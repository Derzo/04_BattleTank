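; Tank Blueprint that binds axis input to orbit its camera rig for aiming.
; AimAzimuth adds local yaw to AzimuthGimbal, while AimElevation sets SpringArm's relative pitch, keeping the two axes on separate components.
; Both scale input by frame delta time and their Azimuth or Elevation rate variable; elevation forces roll and yaw to zero and applies no pitch clamp.
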(event `InputAxis|AimAzimuth`
  (params (AxisValue :type "Float (single-precision)"))
  ;[1 1 1] Camera Input Binding
  (`SceneComponent.K2_AddLocalRotation` (`self.AzimuthGimbal`) (`KismetMathLibrary.MakeRotator` 0.0 0.0 (* AxisValue (`GameplayStatics.GetWorldDeltaSeconds`) (`self.Azimuth`))) false false))

(event `InputAxis|AimElevation`
  (params (AxisValue :type "Float (single-precision)"))
  (bind _springarm (`self.SpringArm`))
  (bind (_relativerotation_roll _relativerotation_pitch) (`KismetMathLibrary.BreakRotator` (`SceneComponent.RelativeRotation` _springarm)))
  ;[1 1 1] Camera Input Binding
  (`SceneComponent.K2_SetRelativeRotation` _springarm (`KismetMathLibrary.MakeRotator` 0.0 (+ _relativerotation_pitch (* AxisValue (`GameplayStatics.GetWorldDeltaSeconds`) (`self.Elevation`)))) false false))

(fn `UserConstructionScript`)